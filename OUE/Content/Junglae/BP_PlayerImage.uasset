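; Scene-capture actor that renders an isolated image of its owner's skeletal mesh, presumably the player character.
; On BeginPlay it finds the owner's SkeletalMeshComponent and sets two scene capture components to show only that mesh.
; It also clears all of that mesh's lighting channels, affecting the live mesh itself.
; EndPlay re-enables only lighting channel 0.
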(event `self.ReceiveBeginPlay`
  (`|ExecutionSequence`
    (:`then_0`
      (bind _output_get (set `self.TargetSkeletalMeshComponent` (`self.GetComponentByClass` (`self.GetOwner`) "/Script/Engine.SkeletalMeshComponent")))
      (`SceneCaptureComponent.ShowOnlyComponent` (`self.CaptureComponent2D`) _output_get)
      (`SceneCaptureComponent.ShowOnlyComponent` (`self.SceneCaptureComponent2D`) _output_get))
    (:`then_1`
      (`PrimitiveComponent.SetLightingChannels` (`self.TargetSkeletalMeshComponent`) false false false))))

(event `self.ReceiveEndPlay`
  (params (EndPlayReason :type "EEndPlayReason Enum" :default "Destroyed"))
  (`PrimitiveComponent.SetLightingChannels` (`self.TargetSkeletalMeshComponent`) true false false))

(fn `UserConstructionScript`)