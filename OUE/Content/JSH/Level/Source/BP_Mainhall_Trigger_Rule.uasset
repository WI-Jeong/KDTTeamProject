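; BP_Mainhall_Trigger_Rule is a trigger-box actor that opens the main hall door once the enemies inside it are gone.
; Box overlap events filter for BP_Enemy_Base1 actors, incrementing EnemyCount on begin overlap and decrementing it on end overlap.
; When an end overlap brings the count to zero, it calls MainHallDoorOpen on the referenced door object and destroys itself, making it a one-shot trigger.
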(event `self.Box.OnComponentBeginOverlap`
  (params (OverlappedComponent :type "PrimitiveComponent Object Reference") (OtherActor :type "Actor Object Reference") (OtherComp :type "PrimitiveComponent Object Reference") (OtherBodyIndex :type Integer) (bFromSweep :type Boolean) (SweepResult :type "HitResult Structure (by ref)"))
  (cast `/Game/SOO/Enemies/AI/BP_Enemy_Base1` OtherActor)
  (`/Engine/EditorBlueprintResources/StandardMacros.IncrementInt` (`self.EnemyCount`)))

(event `self.Box.OnComponentEndOverlap`
  (params (OverlappedComponent :type "PrimitiveComponent Object Reference") (OtherActor :type "Actor Object Reference") (OtherComp :type "PrimitiveComponent Object Reference") (OtherBodyIndex :type Integer))
  (bind _enemycount (`self.EnemyCount`))
  (cast `/Game/SOO/Enemies/AI/BP_Enemy_Base1` OtherActor)
  (`/Engine/EditorBlueprintResources/StandardMacros.DecrementInt` _enemycount
    (:`  `
      (if (== _enemycount 0)
        (`/Game/JSH/Level/Source/OUE_Trigger_Mesh/BP_Mainhole_Rule_Door.MainHall_DoorOpen` (`self.MainHall_DoorOpen`))
        (`self.K2_DestroyActor`)))))

(fn `UserConstructionScript`)