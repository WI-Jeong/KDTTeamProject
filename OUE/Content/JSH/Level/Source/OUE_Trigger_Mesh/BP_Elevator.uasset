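; BP_Elevator is a level elevator that descends a long vertical shaft when something overlaps its trigger component.
; The overlap plays a timeline whose movement track lerps the Elevator component's relative location downward, without sweep.
; The same timeline thins a referenced Exponential Height Fog during the ride, lowering density and scattering distribution while holding height falloff at zero.
; The timeline only plays forward, with no return logic.
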(event `self.ElevatorTrigger.OnComponentBeginOverlap`
  (params (OverlappedComponent :type "PrimitiveComponent Object Reference") (OtherActor :type "Actor Object Reference") (OtherComp :type "PrimitiveComponent Object Reference") (OtherBodyIndex :type Integer) (bFromSweep :type Boolean) (SweepResult :type "HitResult Structure (by ref)"))
  (bind _exponentialheightfog (`/Game/JSH/Level/Source/Fog_Densiy.ExponentialHeightFog` (`self.Fog_Density`)))
  (bind (_direction _elevator_move _fog_density) (`Timeline|타임라인`)
    (:`Update`
      (`|ExecutionSequence`
        (:`then_0`
          (`SceneComponent.K2_SetRelativeLocation` (`self.Elevator`) (`KismetMathLibrary.VLerp` (0.0 0.0 100.0) (0.0 0.0 -4800.0) _elevator_move) false false))
        (:`then_1`
          (`ExponentialHeightFogComponent.SetFogDensity` _exponentialheightfog (`KismetMathLibrary.Lerp` 0.05 0.01 _fog_density))
          (`ExponentialHeightFogComponent.SetVolumetricFogScatteringDistribution` _exponentialheightfog (`KismetMathLibrary.Lerp` 0.2 0.15 _fog_density))
          (`ExponentialHeightFogComponent.SetFogHeightFalloff` _exponentialheightfog 0.0))))))

(fn `UserConstructionScript`)