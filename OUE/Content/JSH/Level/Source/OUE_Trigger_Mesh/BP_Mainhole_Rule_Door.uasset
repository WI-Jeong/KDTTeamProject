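; Main hall door Blueprint that slides open with steam and lighting effects when its MainHall_DoorOpen event is called.
; The event activates two steam door components and plays a timeline.
; The timeline's DoorPosition track drives both the DoorSmallA relative location, lerped from closed to open, and a rising intensity on W.
; The file contains no closing logic, and the construction script is empty.
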(event `MainHall_DoorOpen`
  (`ActorComponent.Activate` (`self.SteamDoor`) false)
  (`ActorComponent.Activate` (`self.SteamDoor2`) false)
  (bind (_direction _doorposition) (`Timeline|Timeline_0`)
    (:`Update`
      (`LightComponent.SetIntensity` (`self.w`) (`KismetMathLibrary.Lerp` 0.0 10000.0 _doorposition))
      (`SceneComponent.K2_SetRelativeLocation` (`self.Door_Small_A`) (`KismetMathLibrary.VLerp` (`self.DoorClosed`) (`self.DoorOpen`) _doorposition) false false))))

(fn `UserConstructionScript`)