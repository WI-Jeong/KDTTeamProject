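; BP_Becorn is a level trigger that lights up the main hall and then opens the enemy doors.
; The first overlap with BecornTrigger fires once, turning on the main hall light.
; A delayed loop then lights each floor pipe light in sequence every tenth of a second.
; After the last one and a one-second pause, every enemy door in the array is triggered open.
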(event `self.BecornTrigger.OnComponentBeginOverlap`
  (params (OverlappedComponent :type "PrimitiveComponent Object Reference") (OtherActor :type "Actor Object Reference") (OtherComp :type "PrimitiveComponent Object Reference") (OtherBodyIndex :type Integer) (bFromSweep :type Boolean) (SweepResult :type "HitResult Structure (by ref)"))
  (bind _currentindex (`self.CurrentIndex`))
  (bind _mainhall_floorlight (`self.MainHall_FloorLight`))
  (`/Engine/EditorBlueprintResources/StandardMacros.DoOnce` false
    (:`Completed`
      (`/Game/JSH/Level/Source/OUE_Trigger_Mesh/Trigger_Light.TriggerOn_Light` (`self.MainHallLight`))
      (`KismetSystemLibrary.Delay` 0.1 :!label _label)
      (`/Game/JSH/Level/Source/OUE_Trigger_Mesh/Trigger_Wall_Pipe_Light1.TriggerOn_PipeLight` (`|GetArrayItem` _mainhall_floorlight _currentindex))
      (bind _result (`/Engine/EditorBlueprintResources/StandardMacros.IncrementInt` _currentindex)
        (:`  `
          (if (== (`KismetArrayLibrary.Array_Length` _mainhall_floorlight) _result)
            (`KismetSystemLibrary.Delay` 1.0)
            (for _array_element (`self.EnemyDoor`)
              (`/Game/JSH/Level/Source/OUE_Trigger_Mesh/BP_EnemyDoor.TriggerOpen` _array_element))
            (else
              (goto _label))))))))

(fn `UserConstructionScript`)