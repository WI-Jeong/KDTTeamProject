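; Base enemy Blueprint that provides melee attack, sword-drawing and patrol route access.
; Attack plays the sword slash montage and fires OnAttackEnd whether it completes or is interrupted.
; WieldSword sets the wielding flag and plays a montage with no asset set in the call, using a notify to spawn BP_Sword on the hand_r socket and firing OnWieldSword on completion.
; WieldWeapon is an empty event, and GetPatrolRoute returns the stored route.
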(event `self.ReceiveBeginPlay`)

(event `Attack`
  (`|PlayMontage` (`self.Mesh`) "/Game/Soo/AnimationsTest/Montage_Sword_Slash.Montage_Sword_Slash"
    (:`OnCompleted`
      _)
    (:`OnInterrupted`
      _))
  (`self.OnAttackEnd`))

(event `WieldWeapon`)

(event `WieldSword`
  (set `self.IsWiedingSword` true)
  (bind _notifyname (`|PlayMontage` (`self.Mesh`))
    (:`OnCompleted`
      (`self.OnWieldSword`))
    (:`OnNotifyBegin`
      (switch `name` _notifyname
        (:`HoldSword`
          (bind _returnvalue (`|SpawnActorFromClass` "/Game/Soo/Weapons/BP_Sword.BP_Sword_C" (`self.GetTransform`) "Undefined" "MultiplyWithRoot" null null))
          (`self.K2_AttachToComponent` _returnvalue (`self.Mesh`) "hand_r" "SnapToTarget" "SnapToTarget" "SnapToTarget" true)
          (set `self.IsWiedingSword` true))))))

(fn `GetPatrolRoute`
  (returns (PatrolRoute :type "/Game/Soo/Enemies/AI/BP_PatrolRoute Object Reference"))
  (return (`self.PatrolRoute`)))

(fn `UserConstructionScript`)